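; Manager actor that imports FBX files at runtime from a file dialog and lets the user inspect and edit the resulting procedural meshes.
; Import callbacks drive a progress notification widget and collect the spawned mesh actors.
; Selecting an actor, node or section opens widgets to hide, isolate or change a section's color, texture and material, with Left Alt enabling multi-select.
; Material swaps reapply the current color and the section's imported diffuse texture.
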(event Custom|DeSelectComponents
  (bind _fbxmainwidget (Variables|Default|GetFBXMainWidget))
  (bind _sectionmaterialwidget (Variables|Default|GetSectionMaterialWidget))
  ;[1 1 1] Unselect Components
  (Class|FBXImportManager|DeSelectAllComponents (Variables|Default|GetCurrentMeshActor) true)
  (Utilities|IsValid _fbxmainwidget
    (:Is%20Valid
      (Widget|RemovefromParent _fbxmainwidget))
    (:Is%20Not%20Valid
      _))
  (Utilities|IsValid _sectionmaterialwidget
    (:Is%20Valid
      (Widget|RemovefromParent _sectionmaterialwidget))))

(event Custom|OnNodeSelected
  (params (NodeID :type Integer))
  (bind _fbxmainwidget (Variables|Default|GetFBXMainWidget))
  (bind _sectionmaterialwidget (Variables|Default|GetSectionMaterialWidget))
  ;[1 1 1] On Node Selected
  (bind _output_get (Variables|Default|SetCurrentNode NodeID))
  (bind _returnvalue (Class|FBXImportManager|SelectNode (Variables|Default|GetCurrentMeshActor) _output_get (Variables|Default|GetSelectSingle)))
  (Utilities|IsValid _fbxmainwidget
    (:Is%20Valid
      (Default|AddSections _fbxmainwidget _returnvalue))
    (:Is%20Not%20Valid
      _))
  (Utilities|IsValid _sectionmaterialwidget
    (:Is%20Valid
      (Widget|RemovefromParent _sectionmaterialwidget))))

(event Custom|OnSectionMaterialChanged
  (params (NewMaterial :type Material%20Interface%20Object%20Reference))
  ;[1 1 1] Update Material Properties of individual section of the Imported Procedural Mesh
  ;;[1 0.3083 0.5208] Update Section Material
  (Variables|Default|SetCurrentColor (.Value (Class|FBXImportManager|GetVectorParamValue (Variables|Default|GetCurrentMeshActor) "BaseColor" (Variables|Default|GetCurrentNode) (Variables|Default|GetCurrentSection))))
  (Class|FBXImportManager|UpdateSectionMaterial (Variables|Default|GetCurrentMeshActor) NewMaterial (Variables|Default|GetCurrentNode) (Variables|Default|GetCurrentSection))
  ;[1 1 1] Get FBXSection Data and use it to restore your original material properties
  (bind (_fbxsection _returnvalue) (Class|FBXImportManager|GetFBXSection (Variables|Default|GetCurrentMeshActor) (Variables|Default|GetCurrentNode) (Variables|Default|GetCurrentSection)))
  (if _returnvalue
    (Class|FBXImportManager|UpdateTextureParam (Variables|Default|GetCurrentMeshActor) "BaseTexture" (.DiffuseTexture (Utilities|Struct|BreakMaterialDynamicStructure (.SectionMaterial (Utilities|Struct|BreakFBXSectionStructure _fbxsection)))) (Variables|Default|GetCurrentNode) (Variables|Default|GetCurrentSection))
    (Class|FBXImportManager|UpdateVectorParam (Variables|Default|GetCurrentMeshActor) "BaseColor" (Variables|Default|GetCurrentColor) (Variables|Default|GetCurrentNode) (Variables|Default|GetCurrentSection))))

(event Custom|Import%20FBX
  (params (HitLocation :type Vector))
  ;[1 0.612 0.5822] Import FBX
  (bind (_filenames _returnvalue) (Class|RuntimeFBXImportBPLibrary|GetOpenFileDialogue "Open FBX Files" "FBX Files (*.fbx)|*.fbx|" false))
  (if _returnvalue
    (Variables|Default|SetHitLocation HitLocation)
    (for _array_element _filenames
      (Class|FBXImportManager|ImportFBXFile _array_element (Variables|Default|GetHitLocation) "/RuntimeFBXImport/Materials/Mat_BaseMaterial.Mat_BaseMaterial" "CustomCollisionFromSource" true))))

(event Custom|SelectMeshComponentEvent
  (params (SelectedComponent :type Primitive%20Component%20Object%20Reference))
  (bind _sectionmaterialwidget (Variables|Default|GetSectionMaterialWidget))
  ;[1 0.3884 0.2584] Select Mesh Component at Hit Location
  (bind (_issection _section _selectedmeshactor) (Class|FBXImportManager|SelectMeshComponent SelectedComponent true))
  (Variables|Default|SetCurrentMeshActor _selectedmeshactor)
  (if _issection
    (Variables|Default|SetCurrentNode (.NodeID (Utilities|Struct|BreakFBXSectionStructure _section)))
    (Variables|Default|SetCurrentSection (.SectionID (Utilities|Struct|BreakFBXSectionStructure _section)))
    (CallFunction|CreateSectionMaterialWidget)
    (else
      ;[1 0.3718 0.332] On FBX Actor Selected
      (Utilities|IsValid _sectionmaterialwidget
        (:Is%20Valid
          (Widget|RemovefromParent _sectionmaterialwidget))
        (:Is%20Not%20Valid
          _))
      (Utilities|IsValid (Variables|Default|GetFBXMainWidget)
        (:Is%20Valid
          (if (UserInterface|Viewport|IsinViewport (Variables|Default|GetFBXMainWidget))
            _
            (else
              (UserInterface|Viewport|AddtoViewport (Variables|Default|GetFBXMainWidget) 0 :!label _label))))
        (:Is%20Not%20Valid
          (bind _returnvalue (UserInterface|CreateWidget "/RuntimeFBXImport/Widgets/UMG_FBXMainWidget.UMG_FBXMainWidget_C" 0 (Utilities|Text|ToText(String) (Variables|/Script/RuntimeFBXImport.FBXMeshActor|GetActorName (Variables|Default|GetCurrentMeshActor)))))
          (Variables|Default|SetFBXMainWidget _returnvalue)
          (CallFunction|BindFBXWidgetsEvents)
          (goto _label)))
      (Default|InitializeNode (Variables|Default|GetFBXMainWidget) (Variables|/Script/RuntimeFBXImport.FBXMeshActor|GetNodeSectionMap (Variables|Default|GetCurrentMeshActor))))))

(event Custom|OnSectionSelected
  (params (NodeID :type Integer) (SectionID :type Integer))
  ;[1 1 1] Section Selected
  (Variables|Default|SetCurrentNode NodeID)
  (Variables|Default|SetCurrentSection SectionID)
  (Class|FBXImportManager|SelectNodeSection (Variables|Default|GetCurrentMeshActor) (Variables|Default|GetCurrentNode) (Variables|Default|GetCurrentSection) (Variables|Default|GetSelectSingle))
  (CallFunction|CreateSectionMaterialWidget))

(event Custom|Bind%20FBXWidgets%20Events
  (Utilities|IsValid (Variables|Default|GetFBXMainWidget)
    (:Is%20Valid
      (EventDispatchers|BindEventtoOnNodeSelected (Variables|Default|GetFBXMainWidget) (delegate Custom|OnNodeSelected))
      (EventDispatchers|BindEventtoOnSectionSelected (Variables|Default|GetFBXMainWidget) (delegate Custom|OnSectionSelected))
      ;[1 0.504 0.3431] Hide/UnHide/Isolate
      (EventDispatchers|BindEventtoOnClicked (Variables|/RuntimeFBXImport/Widgets/UMG_FBXMainWidget.UMG_FBXMainWidget_C|GetbtnHide (Variables|Default|GetFBXMainWidget)) (delegate Custom|OnHide))
      (EventDispatchers|BindEventtoOnClicked (Variables|/RuntimeFBXImport/Widgets/UMG_FBXMainWidget.UMG_FBXMainWidget_C|GetbtnUnHide (Variables|Default|GetFBXMainWidget)) (delegate Custom|OnUnHide))
      (EventDispatchers|BindEventtoOnClicked (Variables|/RuntimeFBXImport/Widgets/UMG_FBXMainWidget.UMG_FBXMainWidget_C|GetbtnIsolate (Variables|Default|GetFBXMainWidget)) (delegate Custom|OnIsolate)))))

(event Custom|OnIsolate
  ;[1 0.504 0.3431] Hide/UnHide/Isolate
  (Class|FBXImportManager|IsolateSelection (Variables|Default|GetCurrentMeshActor)))

(event Custom|OnHide
  ;[1 0.504 0.3431] Hide/UnHide/Isolate
  (Class|FBXImportManager|HideSelection (Variables|Default|GetCurrentMeshActor)))

(event Custom|OnSectionColorChanged
  (params (NewColor :type Linear%20Color%20Structure))
  ;[1 1 1] Update Material Properties of individual section of the Imported Procedural Mesh
  ;;[1 0.1562 0.1661] Update Section Color Parameter
  (Class|FBXImportManager|UpdateVectorParam (Variables|Default|GetCurrentMeshActor) "BaseColor" NewColor (Variables|Default|GetCurrentNode) (Variables|Default|GetCurrentSection)))

(event Custom|OnUnHide
  ;[1 0.504 0.3431] Hide/UnHide/Isolate
  (Class|FBXImportManager|UnHideAll (Variables|Default|GetCurrentMeshActor)))

(event Custom|Create%20Section%20Material%20Widget
  ;[1 1 1] Create Section Material Widget
  (Utilities|IsValid (Variables|Default|GetSectionMaterialWidget)
    (:Is%20Valid
      (if (UserInterface|Viewport|IsinViewport (Variables|Default|GetSectionMaterialWidget))
        _
        (else
          (UserInterface|Viewport|AddtoViewport (Variables|Default|GetSectionMaterialWidget) 0 :!label _label))))
    (:Is%20Not%20Valid
      (bind _returnvalue (UserInterface|CreateWidget "/RuntimeFBXImport/Widgets/UMG_Section.UMG_Section_C"))
      (bind _output_get (Variables|Default|SetSectionMaterialWidget _returnvalue))
      (EventDispatchers|BindEventtoOnSectionColorChanged _output_get (delegate Custom|OnSectionColorChanged))
      (EventDispatchers|BindEventtoOnSectionTextureChanged (Variables|Default|GetSectionMaterialWidget) (delegate Custom|OnSectionTextureChanged))
      (EventDispatchers|BindEventtoOnSectionMaterialChanged (Variables|Default|GetSectionMaterialWidget) (delegate Custom|OnSectionMaterialChanged))
      (goto _label)))
  (Default|UpdateMaterialLayout (Variables|Default|GetSectionMaterialWidget) (.Value (Class|FBXImportManager|GetVectorParamValue (Variables|Default|GetCurrentMeshActor) "BaseColor" (Variables|Default|GetCurrentNode) (Variables|Default|GetCurrentSection))) (Variables|DataTables|GetMaterialLibraryTable) (Variables|DataTables|GetTextureLibraryTable)))

(event Custom|OnSectionTextureChanged
  (params (NewTexture :type Texture%202D%20Object%20Reference))
  ;[1 1 1] Update Material Properties of individual section of the Imported Procedural Mesh
  ;;[0.05805 0.3993 1] Update Section Texture
  (Class|FBXImportManager|UpdateTextureParam (Variables|Default|GetCurrentMeshActor) "BaseTexture" NewTexture (Variables|Default|GetCurrentNode) (Variables|Default|GetCurrentSection)))

(event EventBeginPlay
  ;[1 0.612 0.5822] Begin Importation
  (Variables|Default|SetHitLocation (Transformation|GetActorLocation)))

(event EventOnFBXSectionImported
  (params (ProcMeshSectionMap :type Map%20of%20Integers%20to%20Structs))
  ;[1 1 1] Gather Mesh Data for every imported node
  (bind _keys (Utilities|Map|Keys ProcMeshSectionMap))
  (for _array_element _keys
    (if (.ReturnValue (Utilities|Map|Find ProcMeshSectionMap _array_element))
      _)))

(event EventOnNewFBXImportStarted
  (params (FileName :type String))
  ;[1 0.4561 0.4262] In the event of a new FBX Import
  (Default|CallImportStarted)
  (Utilities|IsValid (Variables|Default|GetNotificationWidget)
    (:Is%20Valid
      (if (UserInterface|Viewport|IsinViewport (Variables|Default|GetNotificationWidget))
        _
        (else
          (UserInterface|Viewport|AddtoViewport (stale _output_get) 0 :!label _label))))
    (:Is%20Not%20Valid
      (bind _returnvalue (UserInterface|CreateWidget "/RuntimeFBXImport/Widgets/UMG_ImportNotification.UMG_ImportNotification_C"))
      (bind _output_get (Variables|Default|SetNotificationWidget _returnvalue))
      (goto _label)))
  (Default|NotifyNewFileImport (Variables|Default|GetNotificationWidget) FileName))

(event EventOnImportCompleted
  (params (CurrentFBXMeshActor :type FBX%20Mesh%20Actor%20Object%20Reference))
  (bind _notificationwidget (Variables|Default|GetNotificationWidget))
  ;[1 0.4561 0.4262] On the completion of an import
  (bind _output_get (Variables|Default|SetCurrentMeshActor CurrentFBXMeshActor))
  (Utilities|Array|Add (Variables|Default|GetMeshActorCollection) _output_get)
  (Utilities|IsValid _notificationwidget
    (:Is%20Valid
      (Default|NotifyImportCompleted _notificationwidget)
      (Default|CallImportCompleted))))

(event EventOnFBXNodeProgressChanged
  (params (NodeIndex :type Integer) (NodeName :type String) (NodeCount :type Integer))
  (bind _notificationwidget (Variables|Default|GetNotificationWidget))
  ;[1 0.4561 0.4262] FBX Node Import Progress
  (Utilities|IsValid _notificationwidget
    (:Is%20Valid
      (Default|NotifyNewNodeProgress _notificationwidget NodeIndex NodeName NodeCount))))

(event EventOnFBXSectionProgressChanged
  (params (SectionIndex :type Integer) (SectionName :type String) (SectionCount :type Integer))
  (bind _notificationwidget (Variables|Default|GetNotificationWidget))
  ;[1 0.4561 0.4262] FBX Section import progress
  (Utilities|IsValid _notificationwidget
    (:Is%20Valid
      (Default|NotifyNewSectionProgress _notificationwidget SectionIndex SectionName SectionCount))))

(event Input|KeyboardEvents|LeftAlt
  (params (Key :type Key%20Structure :default "None"))
  (:Pressed
    (Variables|Default|SetSelectSingle false))
  (:Released
    (Variables|Default|SetSelectSingle true)))

(fn ConstructionScript)